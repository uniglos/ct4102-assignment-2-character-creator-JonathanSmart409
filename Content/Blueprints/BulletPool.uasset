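; BulletPool is a component that pre-spawns a pool of Bp_bullet actors at its owner's location so bullets can be reused.
; On BeginPlay it spawns BulletPoolAmount bullets, disables their collision, binds each one's OnBulletDestroyed event and stores them in the BulletPool array.
; When that event fires, the bullet moves back to the owner and attaches to it.
; The graph contains no logic for taking bullets out of the pool.
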(event `self.ReceiveBeginPlay`
  (for _ (range (+ (`self.BulletPoolAmount`) 1))
    (bind _returnvalue (`|SpawnActorFromClass` "/Game/Blueprints/Bp_bullet.Bp_bullet_C" (`KismetMathLibrary.MakeTransform` (`Actor.K2_GetActorLocation` (`self.GetOwner`))) "Undefined" "MultiplyWithRoot" null null))
    (`PrimitiveComponent.SetCollisionEnabled` (`/Game/Blueprints/Bp_bullet.bullet` _returnvalue) "NoCollision")
    (`Actor.K2_AttachToActor` _returnvalue null "None" "KeepWorld" "KeepWorld" "KeepWorld" true)
    (add `/Game/Blueprints/Bp_bullet.OnBulletDestroyed` _returnvalue (delegate `OnBulletDestroyed_Event`))
    (`KismetArrayLibrary.Array_Add` (`self.BulletPool`) _returnvalue)))

(event `OnBulletDestroyed_Event`
  (params (Bullet :type "/Game/Blueprints/Bp_bullet Object Reference"))
  (bind _returnvalue (`self.GetOwner`))
  (`Actor.K2_SetActorLocation` Bullet (`Actor.K2_GetActorLocation` _returnvalue) false false)
  (`Actor.K2_AttachToActor` Bullet _returnvalue "None" "KeepWorld" "KeepWorld" "KeepWorld" true))