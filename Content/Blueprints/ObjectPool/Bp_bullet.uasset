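; Projectile bullet actor, apparently built for object pooling, that is fired and deactivated without being destroyed.
; Fire sets the projectile velocity, activates the trail and plays a shot sound.
; Overlapping an actor tagged "Clone" zeroes the velocity through DeactivateBullet, then broadcasts OnBulletDestroyed with itself.
; Both Fire and DeactivateBullet set collision to PhysicsOnly, and deactivation leaves the trail and visibility untouched.
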(event `self.bullet.OnComponentBeginOverlap`
  (params (OverlappedComponent :type "PrimitiveComponent Object Reference") (OtherActor :type "Actor Object Reference") (OtherComp :type "PrimitiveComponent Object Reference") (OtherBodyIndex :type Integer) (bFromSweep :type Boolean) (SweepResult :type "HitResult Structure (by ref)"))
  (if (`self.ActorHasTag` OtherActor "Clone")
    (`self.DeactivateBullet`)
    (`self.OnBulletDestroyed` self)))

(event `Fire`
  (params (Velocity :type "Vector Structure"))
  (set `MovementComponent.Velocity` Velocity (`self.ProjectileMovement`))
  (`PrimitiveComponent.SetCollisionEnabled` (`self.bullet`) "PhysicsOnly")
  (`ActorComponent.Activate` (`self.BulletTrail`) false)
  (`GameplayStatics.PlaySoundAtLocation` "/Game/Sounds/Shoot11.Shoot11" (`self.K2_GetActorLocation` self) (struct) 1.0 1.0 0.0 null null null null))

(event `DeactivateBullet`
  (set `MovementComponent.Velocity` (0.0 0.0 0.0) (`self.ProjectileMovement`))
  (`PrimitiveComponent.SetCollisionEnabled` (`self.bullet`) "PhysicsOnly"))

(fn `UserConstructionScript`)