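; Prototype spawner actor that periodically spawns a random actor class from its Items array at its own transform.
; BeginPlay starts a looping timer with a randomly varied initial delay, which fires the Spawn event.
; Each spawn activates the Explosion particle and plays a boom sound at the spawner's location.
; A Clone override only calls its parent, and the Clone call on the spawned actor is left unwired.
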(event `self.ReceiveBeginPlay`
  ; spawns the actor clone with a delay
  (`KismetSystemLibrary.K2_SetTimerDelegate` (delegate `Spawn`) 3.0 true false 2.0 0.7))

(event `Spawn`
  (bind _items (`self.Items`))
  ; spawns the actor clone with a delay
  (bind _returnvalue (`|SpawnActorFromClass` (`|GetArrayItem` _items (`KismetMathLibrary.RandomIntegerInRange` 0 (- (`KismetArrayLibrary.Array_Length` _items) 1))) (`self.GetTransform`) "Undefined" "MultiplyWithRoot" null null))
  ; activates explosion particle and plays sound
  (`ActorComponent.Activate` (`self.Explosion`) false)
  (`GameplayStatics.PlaySoundAtLocation` "/Game/Sounds/Boom4.Boom4" (`self.K2_GetActorLocation`) (struct) 1.0 1.0 0.0 null null null null))

(fn `Clone`
  (params (Transform :type "Transform Structure"))
  (`parent.Clone` Transform))

(fn `UserConstructionScript`
  (`parent.UserConstructionScript`))